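; Noise-emitting actor that makes an AI-audible noise at its own location, with configurable loudness and range and itself as instigator.
; It registers its mesh with the ENTInteractable component on BeginPlay, and each interaction fires one noise through DoNoise.
; RepeatNoises toggles a flag that makes Tick fire the noise every frame.
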(event OnInteract(ENTInteractable)
  (params (Controller :type Player%20Controller%20Object%20Reference) (Pawn :type Pawn%20Object%20Reference) (InteractComponent :type Primitive%20Component%20Object%20Reference))
  (Noise|DoNoise))

(event EventBeginPlay
  (Class|ENTInteractableComponent|AddInteractable (Variables|Default|GetENTInteractable) (Variables|Default|GetActorMesh)))

(event EventTick
  (params (DeltaSeconds :type Float%20%28single-precision%29))
  (if (Variables|Default|GetShouldRepeatNoise)
    (Noise|DoNoise)))

(fn ConstructionScript)

(fn DoNoise
  (Class|Actor|MakeNoise (Variables|Noise|GetNoiseLoundness) self (Transformation|GetActorLocation) (Variables|Noise|GetNoiseRange) "None"))

(fn RepeatNoises
  (Variables|Default|SetShouldRepeatNoise (not (Variables|Default|GetShouldRepeatNoise))))