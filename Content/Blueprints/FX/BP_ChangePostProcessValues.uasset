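; BP_ChangePostProcessValues is a trigger actor that fades a dark post-process effect in and out as actors pass through two boxes.
; Overlapping EntryBox plays a BlendIn timeline that raises DarkPostProcess blend weight toward full.
; Overlapping ExitBox plays a BlendOut timeline that lerps the weight from full back to zero.
; Each box only fires while the weight has not reached its target, and overlaps are not filtered by actor.
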(event OnComponentBeginOverlap(EntryBox)
  (params (OverlappedComponent :type Primitive%20Component%20Object%20Reference) (OtherActor :type Actor%20Object%20Reference) (OtherComp :type Primitive%20Component%20Object%20Reference) (OtherBodyIndex :type Integer) (bFromSweep :type Boolean) (SweepResult :type Hit%20Result%20Structure%20%28by%20ref%29))
  (if (< (Variables|/Script/Engine.PostProcessComponent|GetBlendWeight (Variables|Default|GetDarkPostProcess)) 1.0)
    (bind _nouvelle_piste_0 (Timeline|BlendIn Play)
      (:Update
        (Variables|/Script/Engine.PostProcessComponent|SetBlendWeight (Variables|Default|GetDarkPostProcess) _nouvelle_piste_0)))))

(event OnComponentBeginOverlap(ExitBox)
  (params (OverlappedComponent :type Primitive%20Component%20Object%20Reference) (OtherActor :type Actor%20Object%20Reference) (OtherComp :type Primitive%20Component%20Object%20Reference) (OtherBodyIndex :type Integer) (bFromSweep :type Boolean) (SweepResult :type Hit%20Result%20Structure%20%28by%20ref%29))
  (if (> (Variables|/Script/Engine.PostProcessComponent|GetBlendWeight (Variables|Default|GetDarkPostProcess)) 0.0)
    (bind _nouvelle_piste_0 (Timeline|Blend%20Out Play)
      (:Update
        (Variables|/Script/Engine.PostProcessComponent|SetBlendWeight (Variables|Default|GetDarkPostProcess) (Math|Float|Lerp 1.0 0.0 _nouvelle_piste_0))))))

(fn ConstructionScript)