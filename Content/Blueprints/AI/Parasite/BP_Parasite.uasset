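; BP_Parasite is an AI Blueprint that, as written, only debugs navmesh projection beneath the player.
; Each tick it traces down from the player pawn cached at BeginPlay and projects the hit location onto the navmesh within a cubic query extent.
; It prints whether projection succeeded and draws the query box and projected point.
; A parasite controller reachability check is present but unused.
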(event EventTick
  (params (DeltaSeconds :type Float%20%28single-precision%29))
  (bind _x (Variables|Default|GetX))
  (bind _newvar (Variables|Default|GetNewVar))
  (bind _returnvalue (Transformation|GetActorLocation _newvar))
  (bind _returnvalue_2 (Math|Vector|MakeVector _x _x _x))
  (bind _outhit (Collision|LineTraceByChannel _returnvalue (- _returnvalue "0.000000,0.000000,200.000000") "TraceTypeQuery1" false 0 "None"))
  (Development|PrintString (Utilities|String|ToString(Boolean) (.ReturnValue (AI|Navigation|ProjectPointtoNavigation (.Location (Collision|BreakHitResult _outhit)) 0 0 _returnvalue_2))) true false "(R=0.000000,G=0.660000,B=1.000000,A=1.000000)" 0.0)
  (Rendering|Debug|DrawDebugBox (.Location (Collision|BreakHitResult _outhit)) _returnvalue_2 "(R=1.000000,G=0.022514,B=0.000000,A=1.000000)" "0, 0, 0" 0.0 1.0)
  (Rendering|Debug|DrawDebugPoint (.ProjectedLocation (AI|Navigation|ProjectPointtoNavigation (.Location (Collision|BreakHitResult _outhit)) 0 0 _returnvalue_2)) 15.0 "(R=1.000000,G=0.751051,B=0.000000,A=1.000000)" 0.0))

(event EventBeginPlay
  (Variables|Default|SetNewVar (Game|Player|GetPlayerPawn 0)))

(fn ConstructionScript)