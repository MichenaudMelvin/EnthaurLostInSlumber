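; BP_VeinElement is an actor under the PCG folder with a work-in-progress RaycastDecors function that probes the space above its spline.
; The function samples the spline into five transforms and multi-line-traces upward from each on the Visibility channel.
; Every impact point gets a zero-length sphere trace as an overlap probe, but its result is unused.
; Debug drawing and prints are active, nothing is spawned, and the construction script is empty.
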(fn ConstructionScript)

(fn RaycastDecors
  (bind _frames (Class|GeometryScriptLibraryPolyPathFunctions|SampleSplinetoTransforms (Variables|Default|GetSpline) (Utilities|Struct|MakeGeometryScriptSplineSamplingOptions 5 1.0) (Transformation|GetActorTransform) true))
  (for _array_element _frames
    (bind _outhits (Collision|MultiLineTraceByChannel (.Location (Math|Transform|BreakTransform _array_element)) (+ (.Location (Math|Transform|BreakTransform _array_element)) "0.000000,0.000000,1000.000000") "TraceTypeQuery1" false 0 "ForDuration" false "(R=1.000000,G=0.000000,B=0.000000,A=1.000000)" "(R=0.000000,G=1.000000,B=0.000000,A=1.000000)" 5e+01))
    (Development|PrintString "Raycasting" true true "(R=0.000000,G=0.660000,B=1.000000,A=1.000000)" 1e+01)
    (for _array_element_2 _outhits
      (bind _outhit (Collision|SphereTraceByChannel (.ImpactPoint (Collision|BreakHitResult _array_element_2)) (.ImpactPoint (Collision|BreakHitResult _array_element_2)) 25.0 "TraceTypeQuery1" false 0 "ForDuration" false "(R=1.000000,G=0.175358,B=0.981295,A=1.000000)" "(R=0.303953,G=0.278673,B=1.000000,A=1.000000)" 5e+01)))))