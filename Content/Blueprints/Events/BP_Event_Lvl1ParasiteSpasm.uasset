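; BP_Event_Lvl1ParasiteSpasm is a level 1 event actor that detects when an amber ore's mesh drops below its starting height.
; BeginPlay stores the mesh's initial relative location, and Tick compares its current Z against that value.
; On the first drop it prints "Parasite Spasm" and sets a flag so it fires only once; no spasm effect is implemented beyond the debug print.
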(event EventTick
  (params (DeltaSeconds :type Float%20%28single-precision%29))
  (if (and (< (.Z (Math|Vector|BreakVector (Variables|/Script/Engine.SceneComponent|GetRelativeLocation (Variables|/Script/ENTCore.ENTAmberOre|GetAmberMesh (Variables|Default|GetAmberOre))))) (.Z (Math|Vector|BreakVector (Variables|Default|GetInitialLocation)))) (not (Variables|Default|GetHasBeenTriggered)))
    (Development|PrintString "Parasite Spasm")
    (Variables|Default|SetHasBeenTriggered true)))

(event EventBeginPlay
  (Variables|Default|SetInitialLocation (Variables|/Script/Engine.SceneComponent|GetRelativeLocation (Variables|/Script/ENTCore.ENTAmberOre|GetAmberMesh (Variables|Default|GetAmberOre)))))

(fn ConstructionScript)