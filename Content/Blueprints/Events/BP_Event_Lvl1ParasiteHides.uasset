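; Level 1 scripted event actor that makes the parasite hide when its trigger is first overlapped.
; A one-shot flag guards the overlap, which calls a custom hide event.
; That event caches the parasite's start location and plays a timeline that lerps it straight down on Z, setting the location without sweep so it ignores collision.
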(event OnComponentBeginOverlap(Trigger)
  (params (OverlappedComponent :type Primitive%20Component%20Object%20Reference) (OtherActor :type Actor%20Object%20Reference) (OtherComp :type Primitive%20Component%20Object%20Reference) (OtherBodyIndex :type Integer) (bFromSweep :type Boolean) (SweepResult :type Hit%20Result%20Structure%20%28by%20ref%29))
  (if (not (Variables|Default|GetHasBeenTriggered))
    (Variables|Default|SetHasBeenTriggered true)
    (Development|PrintString "Parasite Hides")
    (CallFunction|ParasiteHides)))

(event Custom|ParasiteHides
  (Variables|Default|SetInitLocation (Transformation|GetActorLocation (Variables|Default|GetParasite)))
  (bind _newtrack_0 (Timeline|ParasiteHIding Play)
    (:Update
      (Transformation|SetActorLocation (Variables|Default|GetParasite) (Math|Vector|MakeVector (.X (Math|Vector|BreakVector (Variables|Default|GetInitLocation))) (.Y (Math|Vector|BreakVector (Variables|Default|GetInitLocation))) (- (.Z (Math|Vector|BreakVector (Variables|Default|GetInitLocation))) (Math|Float|Lerp 0.0 1.6e+03 _newtrack_0))) false false))))

(fn ConstructionScript)