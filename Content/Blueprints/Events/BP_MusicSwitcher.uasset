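; BP_MusicSwitcher is a trigger actor that changes the music as the first-person character moves between its entry and exit boxes.
; Overlapping the entry box applies the next music event and switch value, and overlapping the exit box restores the previous ones.
; A HasEntered flag makes the two boxes alternate, so repeated overlaps of the same box do nothing.
; TryToPlayMusic passes any valid Wwise event or switch to the character's StartMusic and SwitchMusic functions.
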(event OnComponentBeginOverlap(EntryBox)
  (params (OverlappedComponent :type Primitive%20Component%20Object%20Reference) (OtherActor :type Actor%20Object%20Reference) (OtherComp :type Primitive%20Component%20Object%20Reference) (OtherBodyIndex :type Integer) (bFromSweep :type Boolean) (SweepResult :type Hit%20Result%20Structure%20%28by%20ref%29))
  (bind _asbp_first_person_character (Utilities|Casting|CastToBP_FirstPersonCharacter OtherActor))
  (Variables|Default|SetCurrentCharacter _asbp_first_person_character)
  (if (not (Variables|Default|GetHasEntered))
    (Variables|Default|SetHasEntered true)
    (CallFunction|TrytoPlayMusic (Variables|Default|GetNextEvent) (Variables|Default|GetNextMusic))
    (Variables|Default|SetCurrentCharacter 0)))

(event OnComponentBeginOverlap(ExitBox)
  (params (OverlappedComponent :type Primitive%20Component%20Object%20Reference) (OtherActor :type Actor%20Object%20Reference) (OtherComp :type Primitive%20Component%20Object%20Reference) (OtherBodyIndex :type Integer) (bFromSweep :type Boolean) (SweepResult :type Hit%20Result%20Structure%20%28by%20ref%29))
  (bind _asbp_first_person_character (Utilities|Casting|CastToBP_FirstPersonCharacter OtherActor))
  (Variables|Default|SetCurrentCharacter _asbp_first_person_character)
  (if (Variables|Default|GetHasEntered)
    (Variables|Default|SetHasEntered false)
    (CallFunction|TrytoPlayMusic (Variables|Default|GetPreviousEvent) (Variables|Default|GetPreviousMusic))
    (Variables|Default|SetCurrentCharacter 0)))

(fn ConstructionScript)

(fn TrytoPlayMusic
  (params (AkEvent :type Ak%20Audio%20Event%20Object%20Reference) (SwitchValue :type Ak%20Switch%20Value%20Object%20Reference))
  (Utilities|IsValid AkEvent
    (:Is%20Valid
      (Default|StartMusic (Variables|Default|GetCurrentCharacter) AkEvent))
    (:Is%20Not%20Valid
      _))
  (Utilities|IsValid SwitchValue
    (:Is%20Valid
      (Default|SwitchMusic (Variables|Default|GetCurrentCharacter) SwitchValue))))