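; Level 1 event actor that makes a parasite behind a pair of spike doors react, apparently fleeing, once both are lowered.
; Each tick it reads the local height of the middle instance in the small and big doors' instanced static meshes, fetched by child component index.
; When both are below HeightTrigger, it calls TriggerMessage on the parasite and sets HasParasiteFled so this fires only once.
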(event EventTick
  (params (DeltaSeconds :type Float%20%28single-precision%29))
  (bind _heighttrigger (Variables|Default|GetHeightTrigger))
  (bind _asinstanced_static_mesh_component (Utilities|Casting|CastToInstancedStaticMeshComponent (Components|GetChildComponent (Variables|/Script/Engine.Actor|GetRootComponent (Variables|Default|GetSmallSpikeDoor)) 3)))
  (bind _asinstanced_static_mesh_component_2 (Utilities|Casting|CastToInstancedStaticMeshComponent (Components|GetChildComponent (Variables|/Script/Engine.Actor|GetRootComponent (Variables|Default|GetBigSpikeDoor)) 3)))
  (if (Math|Boolean|ANDBoolean (< (.Z (Math|Vector|BreakVector (.Location (Math|Transform|BreakTransform (.OutInstanceTransform (Components|InstancedStaticMesh|GetInstanceTransform _asinstanced_static_mesh_component_2 (/ (Components|InstancedStaticMesh|GetInstanceCount _asinstanced_static_mesh_component_2) 2) false)))))) _heighttrigger) (< (.Z (Math|Vector|BreakVector (.Location (Math|Transform|BreakTransform (.OutInstanceTransform (Components|InstancedStaticMesh|GetInstanceTransform _asinstanced_static_mesh_component (/ (Components|InstancedStaticMesh|GetInstanceCount _asinstanced_static_mesh_component) 2) false)))))) _heighttrigger) (not (Variables|Default|GetHasParasiteFled)))
    (Class|ENTActivation|Trigger(Message) (Variables|Default|GetParasite))
    (Variables|Default|SetHasParasiteFled true)))

(fn ConstructionScript)