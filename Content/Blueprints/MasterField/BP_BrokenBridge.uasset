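; Destructible bridge actor built on a Geometry Collection that collapses when BreakBridge is called and remembers its broken state across saves.
; BreakBridge plays a fall sound, fires a radial field through a MasterField reference after a short delay, then hides the debris and disables its collision.
; Save and load store IsBroken as a byte in the world save keyed by display name, replaying the break on load if set.
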(event Custom|BreakBridge
  (bind _masterfield (Variables|Default|GetMasterField))
  (Utilities|IsValid (Variables|Default|GetMasterField)
    (:Is%20Valid
      (Class|AkGameplayStatics|PostEvent "/Game/WwiseAudio/Events/SFX/Gameplay/AKE_bridgeFall.AKE_bridgeFall")
      (Utilities|FlowControl|Delay 1.0)
      (Variables|/Engine/EditorResources/FieldNodes/FS_MasterField.FS_MasterField_C|SetRadial%20Magnitude _masterfield 5.5e+04)
      (Default|CETrigger _masterfield)
      (Variables|Default|SetIsBroken true)
      (Utilities|FlowControl|Delay 2.5)
      (Rendering|SetVisibility (Variables|Default|GetGeometryCollectionComponent) false false)
      (Collision|SetCollisionEnabled (Variables|Default|GetGeometryCollectionComponent) "NoCollision"))))

(event EventSaveGameElementBP
  (params (CurrentWorldSave :type ENT%20World%20Save%20Object%20Reference))
  (Utilities|Map|Add (Variables|/Script/ENTSaves.ENTWorldSave|GetOtherElements CurrentWorldSave) (Utilities|GetDisplayName self) (Utilities|Struct|MakeENTGameElementData (Utilities|Array|MakeArray (Math|Conversions|ToByte(Integer) (Variables|Default|GetIsBroken))))))

(event EventLoadGameElementBP
  (params (LoadedWorldSave :type ENT%20World%20Save%20Object%20Reference))
  (Utilities|IsValid LoadedWorldSave
    (:Is%20Valid
      (bind _output_get (Variables|Default|SetIsBroken (== (Utilities|Array|Get(acopy) (Utilities|Struct|BreakENTGameElementData (.Value (Utilities|Map|Find (Variables|/Script/ENTSaves.ENTWorldSave|GetOtherElements LoadedWorldSave) (Utilities|GetDisplayName self))))) 1)))
      (if _output_get
        (CallFunction|BreakBridge)))))

(fn ConstructionScript)