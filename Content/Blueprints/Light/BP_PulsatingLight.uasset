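; BP_PulsatingLight is a light Blueprint that animates a point light from a Timeline started on BeginPlay.
; Each Timeline update sets intensity from the scaled track value and applies MaxRadius with a large source radius.
; When the Timeline finishes, intensity drops to the unscaled track value and the light switches to MinRadius with a smaller source radius.
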(event EventBeginPlay
  (bind _main_pointlight (Variables|Default|GetMain_PointLight))
  (bind _main_pointlight_2 (Variables|Default|GetMain_PointLight))
  (bind _main_pointlight_3 (Variables|Default|GetMain_PointLight))
  (bind _newtrack_0 (Timeline|Timeline Play)
    (:Update
      (Rendering|Components|Light|SetIntensity _main_pointlight (* _newtrack_0 1e+04))
      (Rendering|Lighting|SetAttenuationRadius _main_pointlight_3 (Variables|Default|GetMax_Radius))
      (Class|PointLightComponent|SetSourceRadius _main_pointlight_3 2.5e+02))
    (:Finished
      (Rendering|Components|Light|SetIntensity _main_pointlight _newtrack_0)
      (Rendering|Lighting|SetAttenuationRadius _main_pointlight_2 (Variables|Default|GetMin_Radius))
      (Class|PointLightComponent|SetSourceRadius _main_pointlight_2 5e+01))))

(fn ConstructionScript)