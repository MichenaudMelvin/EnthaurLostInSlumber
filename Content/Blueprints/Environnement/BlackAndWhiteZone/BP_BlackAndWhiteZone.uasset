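; Black-and-white zone actor that drives a post-process material using its own location and a radius, presumably to desaturate that area.
; The construction script creates a dynamic instance of the first post-process material, writes it back into that slot at full weight and stores it.
; It then feeds the actor's location and Radius into the instance's Position and Radius parameters.
; Nothing updates at runtime, as the event graph holds only disabled placeholders.
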(event Collision|EventActorBeginOverlap
  (params (OtherActor :type Actor%20Object%20Reference)))

(event EventTick
  (params (DeltaSeconds :type Float%20%28single-precision%29)))

(fn ConstructionScript
  (bind _returnvalue (Rendering|Material|CreateDynamicMaterialInstance (Utilities|GetMaterial) "None" "None" :!class /Script/Engine.KismetMaterialLibrary))
  (Utilities|SetMaterial 0 _returnvalue)
  (Rendering|Material|SetVectorParameterValue _returnvalue "Position" (Math|Conversions|ToLinearColor(Vector) (Transformation|GetActorLocation)) :!class /Script/Engine.MaterialInstanceDynamic)
  (Rendering|Material|SetScalarParameterValue _returnvalue "Radius" (Variables|Default|GetRadius) :!class /Script/Engine.MaterialInstanceDynamic)
  (Variables|Default|SetMaterial _returnvalue))