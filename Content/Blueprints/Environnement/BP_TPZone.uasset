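; BP_TPZone is a teleport zone that moves the first-person character to StartTransform when it overlaps the collision component.
; When UseStartTransform is set, the construction script derives StartTransform from the level's PlayerStart, converted into the zone's local space with unit scale.
; The overlap applies that value directly through SetActorTransform, without converting it back to world space.
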(event OnComponentBeginOverlap(CollisionComponent)
  (params (OverlappedComponent :type Primitive%20Component%20Object%20Reference) (OtherActor :type Actor%20Object%20Reference) (OtherComp :type Primitive%20Component%20Object%20Reference) (OtherBodyIndex :type Integer) (bFromSweep :type Boolean) (SweepResult :type Hit%20Result%20Structure%20%28by%20ref%29))
  (if (Class|GameplayStatics|ObjectIsA OtherActor "/Game/Blueprints/Player/BP_FirstPersonCharacter.BP_FirstPersonCharacter_C")
    (Transformation|SetActorTransform OtherActor (Variables|Transform|GetStartTransform))))

(event EventBeginPlay)

(fn ConstructionScript
  (Transform|SetTransform))

(fn SetTransform
  (if (Variables|Transform|GetUseStartTransform)
    (bind _returnvalue (Actor|GetActorOfClass "/Script/Engine.PlayerStart"))
    (LocalVariables|SetActor _returnvalue)
    (Variables|Transform|SetStartTransform (Math|Transform|MakeTransform (Math|Transform|InverseTransformLocation (Transformation|GetActorTransform) (Transformation|GetActorLocation (LocalVariables|GetActor))) (Math|Transform|InverseTransformRotation (Transformation|GetActorTransform) (Transformation|GetActorRotation (LocalVariables|GetActor)))))))