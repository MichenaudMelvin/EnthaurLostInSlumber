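; BP_WeakZone is a weakened area with a black-and-white post-process and its own ambience while a pawn is inside, until it is cured.
; Construction feeds zone position and radius to a dynamic material, and scatters foliage meshes around interaction points using seeded random offsets and ground traces.
; Foliage starts at zero scale on BeginPlay; on cure, it tweens to full size with a growth sound, then the zone is destroyed.
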(event OnComponentBeginOverlap(BoxComponent)
  (params (OverlappedComponent :type Primitive%20Component%20Object%20Reference) (OtherActor :type Actor%20Object%20Reference) (OtherComp :type Primitive%20Component%20Object%20Reference) (OtherBodyIndex :type Integer) (bFromSweep :type Boolean) (SweepResult :type Hit%20Result%20Structure%20%28by%20ref%29))
  (if (Class|GameplayStatics|ObjectIsA OtherActor "/Script/Engine.Pawn")
    (Class|AkGameplayStatics|PostEvent "/Game/WwiseAudio/Event/AMB/AMB_WEAKENEDZONE.AMB_WEAKENEDZONE")))

(event OnComponentEndOverlap(BoxComponent)
  (params (OverlappedComponent :type Primitive%20Component%20Object%20Reference) (OtherActor :type Actor%20Object%20Reference) (OtherComp :type Primitive%20Component%20Object%20Reference) (OtherBodyIndex :type Integer))
  (if (Class|GameplayStatics|ObjectIsA OtherActor "/Script/Engine.Pawn")
    (Class|AkGameplayStatics|PostEvent "/Game/WwiseAudio/Event/AMB/AMB_GAMEPLAY.AMB_GAMEPLAY")))

(event Custom|OnCure_Event
  (Class|AkGameplayStatics|PostEvent "/Game/WwiseAudio/Event/SFX/Play_SFX_Plant_Growth.Play_SFX_Plant_Growth")
  (bind _value (|TweenVector "0, 0, 0" (Variables|Foliage|GetDefaultFoliageScale) 3.0 "OutExpo")
    (:ApplyEasing
      (for _array_element (Variables|Foliage|GetFoliageMeshes)
        (Transformation|SetWorldScale3D _array_element _value)))
    (:OnComplete
      (Class|WeakZone|DestroyZone))))

(event EventBeginPlay
  (for _array_element (Variables|Foliage|GetFoliageMeshes)
    (Transformation|SetWorldScale3D _array_element "0, 0, 0"))
  (EventDispatchers|AssignOnCure (EventDispatchers|CreateEvent :!event Custom|OnCure_Event))
  (Class|WeakZone|CheckifEveryInteractionsPointActive))

(fn ConstructionScript
  (bind _returnvalue (Rendering|Material|CreateDynamicMaterialInstance "/Game/Art/Shaders/M_BlackAndWhiteZone.M_BlackAndWhiteZone" "None" "None" :!class /Script/Engine.KismetMaterialLibrary))
  (bind _output_get (Variables|Default|SetMaterialBlackAndWhite _returnvalue))
  (Utilities|Array|SetArrayElem (Utilities|Struct|BreakWeightedBlendables (Utilities|Struct|BreakPostProcessSettings (Variables|/Script/Engine.PostProcessComponent|GetSettings (Variables|Default|GetBlackAndWhiteShader)))) 0 (Utilities|Struct|MakeWeightedBlendable 1.0 _output_get))
  (Rendering|Material|SetScalarParameterValue _output_get "Radius" (Utilities|GetRadius) :!class /Script/Engine.MaterialInstanceDynamic)
  (Rendering|Material|SetVectorParameterValue _output_get "Position" (Math|Conversions|ToLinearColor(Vector) (Transformation|GetActorLocation)) :!class /Script/Engine.MaterialInstanceDynamic)
  (Foliage|CreateFoliagesMeshes))

(fn CreateFoliagesMeshes
  (bind _foliagerandomoffset (Variables|Foliage|GetFoliageRandomOffset))
  (bind (_lowerbound _upperbound) (Utilities|Struct|BreakFloatRange _foliagerandomoffset))
  (for _array_element (Variables|Default|GetInteractionPoints)
    (for _index (range 0 (Variables|Foliage|GetNumberOfMeshesByInteractionsPoints))
      (bind (_outhit _returnvalue) (Collision|LineTraceForObjects (Math|Vector|MakeVector (.X (Math|Vector|BreakVector (+ (.Location (Math|Transform|BreakTransform (Math|Transform|ComposeTransforms (.Transform (Utilities|Struct|BreakInteractionPoints _array_element)) (Transformation|GetActorTransform)))) (* (Math|Random|RandomUnitVectorfromStream (Variables|Foliage|GetSeed)) (Math|Random|RandomFloatinRangefromStream (Variables|Foliage|GetSeed) (Utilities|Struct|BreakFloatRangeBound _lowerbound) (Utilities|Struct|BreakFloatRangeBound _upperbound)))))) (.Y (Math|Vector|BreakVector (+ (.Location (Math|Transform|BreakTransform (Math|Transform|ComposeTransforms (.Transform (Utilities|Struct|BreakInteractionPoints _array_element)) (Transformation|GetActorTransform)))) (* (Math|Random|RandomUnitVectorfromStream (Variables|Foliage|GetSeed)) (Math|Random|RandomFloatinRangefromStream (Variables|Foliage|GetSeed) (Utilities|Struct|BreakFloatRangeBound _lowerbound) (Utilities|Struct|BreakFloatRangeBound _upperbound)))))) (+ (.Z (Math|Vector|BreakVector (.Location (Math|Transform|BreakTransform (Math|Transform|ComposeTransforms (.Transform (Utilities|Struct|BreakInteractionPoints _array_element)) (Transformation|GetActorTransform)))))) (Variables|Foliage|GetTraceLength))) (Math|Vector|MakeVector (.X (Math|Vector|BreakVector (+ (.Location (Math|Transform|BreakTransform (Math|Transform|ComposeTransforms (.Transform (Utilities|Struct|BreakInteractionPoints _array_element)) (Transformation|GetActorTransform)))) (* (Math|Random|RandomUnitVectorfromStream (Variables|Foliage|GetSeed)) (Math|Random|RandomFloatinRangefromStream (Variables|Foliage|GetSeed) (Utilities|Struct|BreakFloatRangeBound _lowerbound) (Utilities|Struct|BreakFloatRangeBound _upperbound)))))) (.Y (Math|Vector|BreakVector (+ (.Location (Math|Transform|BreakTransform (Math|Transform|ComposeTransforms (.Transform (Utilities|Struct|BreakInteractionPoints _array_element)) (Transformation|GetActorTransform)))) (* (Math|Random|RandomUnitVectorfromStream (Variables|Foliage|GetSeed)) (Math|Random|RandomFloatinRangefromStream (Variables|Foliage|GetSeed) (Utilities|Struct|BreakFloatRangeBound _lowerbound) (Utilities|Struct|BreakFloatRangeBound _upperbound)))))) (- (.Z (Math|Vector|BreakVector (.Location (Math|Transform|BreakTransform (Math|Transform|ComposeTransforms (.Transform (Utilities|Struct|BreakInteractionPoints _array_element)) (Transformation|GetActorTransform)))))) (Variables|Foliage|GetTraceLength))) (Utilities|Array|MakeArray "ObjectTypeQuery1" "ObjectTypeQuery2") false 0 "None"))
      (if _returnvalue
        (bind _returnvalue_2 (AddComponent|AddStaticMeshComponent false (Math|Transform|MakeTransform (Math|Transform|InverseTransformLocation (Transformation|GetActorTransform) (.Location (Collision|BreakHitResult _outhit))) (Math|Rotator|MakeRotator 0.0 0.0 (Math|Random|RandomFloatinRangefromStream (Variables|Foliage|GetSeed) 0.0 3.6e+02)) (Variables|Foliage|GetDefaultFoliageScale))))
        (Utilities|Array|Add (Variables|Foliage|GetFoliageMeshes) _returnvalue_2))))
  (return))