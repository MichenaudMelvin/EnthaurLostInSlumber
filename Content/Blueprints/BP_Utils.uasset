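; BP_Utils is a utility Blueprint that converts an object to a package name and loads an asset back from one.
; GetPackageName rebuilds the name by cutting the object's path at the first match of its display name and re-appending that name.
; LoadAssetByPackageName queries the Asset Registry, including in-memory assets, and loads the first result without checking that one exists.
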(fn GetPackageName
  (params (Object :type Object%20Object%20Reference))
  (bind _returnvalue (Utilities|GetDisplayName Object))
  (return (Utilities|String|StringToName (Utilities|String|Append (.LeftS (Utilities|String|Split (Class|KismetSystemLibrary|GetPathName Object) _returnvalue)) _returnvalue))))

(fn LoadAssetbyPackageName
  (params (PackageName :type Name))
  (bind _outassetdata (Class|AssetRegistry|GetAssetsbyPackageName (Class|AssetRegistryHelpers|GetAssetRegistry) PackageName false true))
  (return (Class|AssetRegistryHelpers|GetAsset (Utilities|Array|Get(acopy) _outassetdata))))