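; Flickering light actor that switches a spot light and a point light between a base and a minimum intensity.
; From BeginPlay, a retriggerable delay of random length between Min and Max feeds a FlipFlop that alternately sets both lights to the low and base intensity.
; Each branch loops back into the delay, so the irregular flicker repeats indefinitely without using Tick.
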(event EventBeginPlay
  (bind _main_spotlight (Variables|Default|GetMain_SpotLight))
  (Utilities|FlowControl|RetriggerableDelay (Math|Random|RandomFloatinRange (Variables|Default|GetMin) (Variables|Default|GetMax)) :!label _label)
  (Utilities|FlowControl|FlipFlop
    (:A
      (Rendering|Components|Light|SetIntensity _main_spotlight (Variables|Default|GetMin_Intensity))
      (goto _label))
    (:B
      (Rendering|Components|Light|SetIntensity _main_spotlight (Variables|Default|GetBase_Intensity))
      (goto _label))))

(fn ConstructionScript)