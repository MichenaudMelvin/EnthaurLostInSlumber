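; BP_LevelLoader is a trigger actor that streams sublevels in and out at a boundary between areas.
; Overlapping EntryBox loads NextLevels and unloads PreviousLevels, while ExitBox does the reverse, with no filter on the overlapping actor.
; LoadLevels and UnloadLevels step through their arrays by calling themselves with an index counter, using non-blocking latent stream calls and making loaded levels visible.
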(event OnComponentBeginOverlap(EntryBox)
  (params (OverlappedComponent :type Primitive%20Component%20Object%20Reference) (OtherActor :type Actor%20Object%20Reference) (OtherComp :type Primitive%20Component%20Object%20Reference) (OtherBodyIndex :type Integer) (bFromSweep :type Boolean) (SweepResult :type Hit%20Result%20Structure%20%28by%20ref%29))
  (Variables|Default|SetLoadIndex 0)
  (Variables|Default|SetUnloadIndex 0)
  (CallFunction|LoadLevels (Variables|Default|GetNext_Levels))
  (CallFunction|UnloadLevels (Variables|Default|GetPrevious_Levels)))

(event OnComponentBeginOverlap(ExitBox)
  (params (OverlappedComponent :type Primitive%20Component%20Object%20Reference) (OtherActor :type Actor%20Object%20Reference) (OtherComp :type Primitive%20Component%20Object%20Reference) (OtherBodyIndex :type Integer) (bFromSweep :type Boolean) (SweepResult :type Hit%20Result%20Structure%20%28by%20ref%29))
  (Variables|Default|SetLoadIndex 0)
  (Variables|Default|SetUnloadIndex 0)
  (CallFunction|LoadLevels (Variables|Default|GetPrevious_Levels))
  (CallFunction|UnloadLevels (Variables|Default|GetNext_Levels)))

(event Custom|LoadLevels
  (params (LevelsToLoad :type Array%20of%20Names))
  (Game|LoadStreamLevel(byName) (Utilities|Array|Get(acopy) LevelsToLoad (Variables|Default|GetLoadIndex)) true)
  (if (< (Variables|Default|GetLoadIndex) (- (Utilities|Array|Length LevelsToLoad) 1))
    (Math|Integer|IncrementInt (Variables|Default|GetLoadIndex)
      (:%20%20
        (CallFunction|LoadLevels LevelsToLoad)))))

(event Custom|UnloadLevels
  (params (LevelsToUnload :type Array%20of%20Names))
  (Game|UnloadStreamLevel(byName) (Utilities|Array|Get(acopy) LevelsToUnload (Variables|Default|GetUnloadIndex)) false)
  (if (< (Variables|Default|GetUnloadIndex) (- (Utilities|Array|Length LevelsToUnload) 1))
    (Math|Integer|IncrementInt (Variables|Default|GetUnloadIndex)
      (:%20%20
        (CallFunction|UnloadLevels LevelsToUnload)))))

(event EventBeginPlay)

(event Collision|EventActorBeginOverlap
  (params (OtherActor :type Actor%20Object%20Reference)))

(event EventTick
  (params (DeltaSeconds :type Float%20%28single-precision%29)))

(fn ConstructionScript)