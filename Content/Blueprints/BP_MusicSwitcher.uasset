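; BP_MusicSwitcher is a level trigger that changes the music as the player moves through a boundary.
; EntryBox and ExitBox overlaps toggle a HasEntered flag, so each side fires only after the other.
; Entering sends the Next event and music to BP_FirstPersonCharacter through StartMusic and SwitchMusic, and exiting sends the Previous pair, skipping any unset value.
; The overlapping actor is not checked; the calls always target player pawn 0.
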(event OnComponentBeginOverlap(EntryBox)
  (params (OverlappedComponent :type Primitive%20Component%20Object%20Reference) (OtherActor :type Actor%20Object%20Reference) (OtherComp :type Primitive%20Component%20Object%20Reference) (OtherBodyIndex :type Integer) (bFromSweep :type Boolean) (SweepResult :type Hit%20Result%20Structure%20%28by%20ref%29))
  (bind _next_music (Variables|Default|GetNext_Music))
  (bind _nextevent (Variables|Default|GetNextEvent))
  (if (not (Variables|Default|GetHasEntered))
    (Variables|Default|SetHasEntered true)
    (bind _asbp_first_person_character (Utilities|Casting|CastToBP_FirstPersonCharacter (Game|Player|GetPlayerPawn 0)))
    (if (Utilities|IsValid _nextevent)
      (Default|StartMusic _asbp_first_person_character _nextevent))
    (if (Utilities|IsValid _next_music)
      (Default|SwitchMusic _asbp_first_person_character _next_music))))

(event OnComponentBeginOverlap(ExitBox)
  (params (OverlappedComponent :type Primitive%20Component%20Object%20Reference) (OtherActor :type Actor%20Object%20Reference) (OtherComp :type Primitive%20Component%20Object%20Reference) (OtherBodyIndex :type Integer) (bFromSweep :type Boolean) (SweepResult :type Hit%20Result%20Structure%20%28by%20ref%29))
  (bind _previousevent (Variables|Default|GetPreviousEvent))
  (bind _previous_music (Variables|Default|GetPrevious_Music))
  (if (Variables|Default|GetHasEntered)
    (Variables|Default|SetHasEntered false)
    (bind _asbp_first_person_character (Utilities|Casting|CastToBP_FirstPersonCharacter (Game|Player|GetPlayerPawn 0)))
    (if (Utilities|IsValid _previousevent)
      (Default|StartMusic _asbp_first_person_character _previousevent))
    (if (Utilities|IsValid _previous_music)
      (Default|SwitchMusic _asbp_first_person_character _previous_music))))

(event EventBeginPlay)

(event Collision|EventActorBeginOverlap
  (params (OtherActor :type Actor%20Object%20Reference)))

(event EventTick
  (params (DeltaSeconds :type Float%20%28single-precision%29)))

(fn ConstructionScript)