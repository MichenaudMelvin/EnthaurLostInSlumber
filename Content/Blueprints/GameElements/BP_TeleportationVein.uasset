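; BP_TeleportationVein is a trigger that moves the player to another level when the first-person character enters its box collider.
; On overlap it hides the HUD, forces the player's state machine to Idle with camera movement off, and locks all states.
; It then optionally switches music, saves the world to slot 0, spawns a transition widget targeting the configured map, and destroys itself.
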(event OnComponentBeginOverlap(BoxCollider)
  (params (OverlappedComponent :type Primitive%20Component%20Object%20Reference) (OtherActor :type Actor%20Object%20Reference) (OtherComp :type Primitive%20Component%20Object%20Reference) (OtherBodyIndex :type Integer) (bFromSweep :type Boolean) (SweepResult :type Hit%20Result%20Structure%20%28by%20ref%29))
  (bind _asbp_first_person_character (Utilities|Casting|CastToBP_FirstPersonCharacter OtherActor))
  (Variables|Character|SetFirstPersonCharacter _asbp_first_person_character)
  (Class|ENTHUDManager|HideHUD (Subsystems|GetENTHUDManager))
  (bind _returnvalue (Class|ENTCharacterStateMachine|ChangeState (Variables|/Script/ENTCore.ENTDefaultCharacter|GetStateMachine (Variables|Character|GetFirstPersonCharacter)) "Idle"))
  (Variables|/Script/ENTCore.ENTCharacterState|SetbAllowCameraMovement _returnvalue false)
  (Class|ENTCharacterStateMachine|LockAllStates (Variables|/Script/ENTCore.ENTDefaultCharacter|GetStateMachine (Variables|Character|GetFirstPersonCharacter)) true)
  (Utilities|IsValid (Variables|Music|GetMusicSwitchToStop)
    (:Is%20Valid
      (Default|SwitchMusic (Variables|Character|GetFirstPersonCharacter) (Variables|Music|GetMusicSwitchToStop)))
    (:Is%20Not%20Valid
      _))
  (Class|ENTSaveSubsystem|SavetoSlot (Subsystems|GetENTWorldSaveSubsystem))
  (bind _returnvalue_2 (UserInterface|CreateWidget "/Game/Blueprints/UI/HUD/WBP_Transition.WBP_Transition_C" 0 (Variables|Default|GetMapToLoad) 0.8))
  (UserInterface|Viewport|AddtoViewport _returnvalue_2 0)
  (Actor|DestroyActor))

(fn ConstructionScript)