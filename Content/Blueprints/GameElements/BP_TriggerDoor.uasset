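; BP_TriggerDoor is a trigger that closes a referenced SpikeDoor when the first-person character enters its box with the lantern mesh visible.
; On overlap it stores the door's position and plays the CloseDoor timeline, lerping a Z offset that moves the door upward from there.
; The IsDoorClosed flag, set during timeline updates, makes it one-shot; nothing here reopens the door.
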(event OnComponentBeginOverlap(Box)
  (params (OverlappedComponent :type Primitive%20Component%20Object%20Reference) (OtherActor :type Actor%20Object%20Reference) (OtherComp :type Primitive%20Component%20Object%20Reference) (OtherBodyIndex :type Integer) (bFromSweep :type Boolean) (SweepResult :type Hit%20Result%20Structure%20%28by%20ref%29))
  (bind _asbp_first_person_character (Utilities|Casting|CastToBP_FirstPersonCharacter OtherActor))
  (if (Rendering|IsVisible (Variables|/Game/Blueprints/Player/BP_FirstPersonCharacter.BP_FirstPersonCharacter_C|GetLanternMesh _asbp_first_person_character))
    (if (not (Variables|Default|GetisDoorClosed))
      (Variables|Default|SetInit%20Position (Transformation|GetActorLocation (Variables|Default|GetSpikeDoor)))
      (bind _doorposition (Timeline|CloseDoor Play)
        (:Update
          (Transformation|SetActorLocation (Variables|Default|GetSpikeDoor) (Math|Vector|MakeVector (.X (Math|Vector|BreakVector (Variables|Default|GetInit%20Position))) (.Y (Math|Vector|BreakVector (Variables|Default|GetInit%20Position))) (+ (Math|Float|Lerp 0.0 5.5e+02 _doorposition) (.Z (Math|Vector|BreakVector (Variables|Default|GetInit%20Position))))) false false)
          (Variables|Default|SetisDoorClosed true))))))

(fn ConstructionScript)