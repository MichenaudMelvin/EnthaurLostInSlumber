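; Vein teleporter actor that moves the player to another level when interacted with.
; An Interaction component registers a Box as interactable, and interacting blends the controller's view to this actor.
; Once the blend delay ends it plays AnimSequence.
; FinishEvent, grouped as a sequencer event, adds a WB_Transition widget to the viewport, waits briefly, then opens MapToLoad.
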(event OnInteract(Interaction)
  (params (Controller :type Player%20Controller%20Object%20Reference) (Pawn :type Pawn%20Object%20Reference) (InteractComponent :type Primitive%20Component%20Object%20Reference))
  (Game|Player|SetViewTargetwithBlend Controller self (Variables|Default|GetCameraBlendDuration) "VTBlend_Linear" 0.0 false)
  (Utilities|FlowControl|Delay (Variables|Default|GetCameraBlendDuration))
  (Class|ActorSequenceComponent|PlaySequence (Variables|Default|GetAnimSequence)))

(event EventBeginPlay
  (Class|InteractableComponent|AddInteractable (Variables|Default|GetInteraction) (Variables|Default|GetBox)))

(event Custom|FinishEvent
  (bind _returnvalue (UserInterface|CreateWidget "/Game/Blueprints/UI/LevelNavigation/WB_Transition.WB_Transition_C"))
  (UserInterface|Viewport|AddtoViewport _returnvalue 0)
  (Utilities|FlowControl|Delay 2.0)
  (Game|OpenLevel(byObjectReference) (Variables|Default|GetMapToLoad)))

(fn ConstructionScript)