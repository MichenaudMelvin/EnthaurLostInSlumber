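; Trigger zone that shows a tutorial widget while the first-person character stands inside its box.
; On begin overlap it creates and displays a WBP_Tutorial, plays its show animation and fills in the zone's Icon and Description.
; On end overlap it plays the disappear animation, waits a second, then removes the widget and clears the reference.
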(event OnComponentBeginOverlap(Box)
  (params (OverlappedComponent :type Primitive%20Component%20Object%20Reference) (OtherActor :type Actor%20Object%20Reference) (OtherComp :type Primitive%20Component%20Object%20Reference) (OtherBodyIndex :type Integer) (bFromSweep :type Boolean) (SweepResult :type Hit%20Result%20Structure%20%28by%20ref%29))
  (Utilities|Casting|CastToBP_FirstPersonCharacter OtherActor)
  (bind _returnvalue (UserInterface|CreateWidget "/Game/Blueprints/UI/HUD/WBP_Tutorial.WBP_Tutorial_C"))
  (UserInterface|Viewport|AddtoViewport _returnvalue 0)
  (bind _output_get (Variables|Default|SetUI _returnvalue))
  (UserInterface|Animation|PlayAnimation _output_get (Variables|/Game/Blueprints/UI/HUD/WBP_Tutorial.WBP_Tutorial_C|GetTutorialShow _output_get) 0.0 1 "Forward" 1.0 false)
  (Appearance|SetBrushfromTexture (Variables|/Game/Blueprints/UI/HUD/WBP_Tutorial.WBP_Tutorial_C|GetTutorialIcon _output_get) (Variables|Default|GetIcon) false)
  (Rendering|Components|TextRender|SetText (Variables|/Game/Blueprints/UI/HUD/WBP_Tutorial.WBP_Tutorial_C|GetTutorialDescription _output_get) (Variables|Default|GetDescription)))

(event OnComponentEndOverlap(Box)
  (params (OverlappedComponent :type Primitive%20Component%20Object%20Reference) (OtherActor :type Actor%20Object%20Reference) (OtherComp :type Primitive%20Component%20Object%20Reference) (OtherBodyIndex :type Integer))
  (Utilities|Casting|CastToBP_FirstPersonCharacter OtherActor)
  (Utilities|IsValid (Variables|Default|GetUI)
    (:Is%20Valid
      (UserInterface|Animation|PlayAnimation (Variables|Default|GetUI) (Variables|/Game/Blueprints/UI/HUD/WBP_Tutorial.WBP_Tutorial_C|GetTutorialDisapear (Variables|Default|GetUI)) 0.0 1 "Forward" 1.0 false)
      (Utilities|FlowControl|Delay 1.0)
      (Widget|RemovefromParent (Variables|Default|GetUI))
      (Variables|Default|SetUI 0))))

(fn ConstructionScript)