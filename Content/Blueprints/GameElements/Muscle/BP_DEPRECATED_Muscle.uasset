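; Deprecated muscle actor that toggles between solid and soft, acting as a launch pad when soft.
; Interacting or triggering flips physical material, material tint and button position unless locked or in a weak zone, with a timer for non-default states.
; Fast impacts on soft muscle squash the mesh along a curve, carrying tracked actors down.
; At full compression it launches them along its up vector, then springs back.
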(event OnInteract(Interactable)
  (params (Controller :type Player%20Controller%20Object%20Reference) (Pawn :type Pawn%20Object%20Reference) (InteractComponent :type Primitive%20Component%20Object%20Reference))
  (Interaction|ToggleMuscleSolidity))

(event OnComponentHit(StaticMesh)
  (params (HitComponent :type Primitive%20Component%20Object%20Reference) (OtherActor :type Actor%20Object%20Reference) (OtherComp :type Primitive%20Component%20Object%20Reference) (NormalImpulse :type Vector :default "0, 0, 0") (Hit :type Hit%20Result%20Structure%20%28by%20ref%29))
  (Physics|HitMuscle OtherActor))

(event Custom|StartDeformation
  (Variables|Deformation|SetDeformationDirection 1)
  (Variables|Deformation|SetTriggerDeformation true))

(event Custom|EndDeformation
  (Variables|Deformation|SetDeformationDirection -1)
  (Variables|Deformation|SetTriggerDeformation true))

(event Custom|UpdateColorFeedback
  (Utilities|IsValid (Variables|Materials|GetDynamicMaterial)
    (:Is%20Valid
      (if (Variables|Deformation|GetIsSolid)
        (bind _floatvalue (Timeline|FeedbackUpdate Play)
          (:Update
            (Rendering|Material|SetScalarParameterValue (Variables|Materials|GetDynamicMaterial) "LerpValue" _floatvalue :!class /Script/Engine.MaterialInstanceDynamic)))
        (else
          (Timeline|FeedbackUpdate Reverse))))))

(event Custom|UpdateBuzzer
  (bind _button (Variables|Default|GetButton))
  (bind _relativelocation (Variables|/Script/Engine.SceneComponent|GetRelativeLocation _button))
  (if (Variables|Deformation|GetIsSolid)
    (bind _value (|TweenFloat -1e+01 0.0 0.5 "InBack")
      (:ApplyEasing
        (Transformation|SetRelativeLocation _button (Math|Vector|MakeVector (.x _relativelocation) (.y _relativelocation) _value) false false)))
    (else
      (bind _value_2 (|TweenFloat 0.0 -1e+01 0.5 "OutBack")
        (:ApplyEasing
          (Transformation|SetRelativeLocation _button (Math|Vector|MakeVector (.x _relativelocation) (.y _relativelocation) _value_2) false false))))))

(event EventOnExitWeakZone
  (Variables|WeakZone|SetInWeakZone false))

(event EventOnEnterWeakZone
  (params (bIsZoneActive :type Boolean))
  (Variables|WeakZone|SetInWeakZone true))

(event EventTick
  (params (DeltaSeconds :type Float%20%28single-precision%29))
  (Deformation|DeformMesh DeltaSeconds))

(event EventBeginPlay
  (bind _staticmesh (Variables|Default|GetStaticMesh))
  (bind _staticmesh_2 (Variables|/Script/Engine.StaticMeshComponent|GetStaticMesh _staticmesh))
  (bind _returnvalue (StaticMesh|GetBoundingBox _staticmesh_2))
  (bind (_min _max) (Utilities|Struct|BreakBox _returnvalue))
  (Class|InteractableComponent|AddInteractable (Variables|Default|GetInteractable) (Variables|Default|GetMuscleActivation))
  (Variables|Deformation|SetDefaultSolidityState (Variables|Deformation|GetIsSolid))
  (Interaction|UpdateMuscleSolidity)
  (Variables|Dimensions|SetMeshZUnit (* (.Z (Math|Vector|BreakVector (- _max _min))) 0.5))
  (bind _returnvalue_2 (Rendering|Material|CreateDynamicMaterialInstance (Variables|Default|GetStaticMesh) 0 (Rendering|Material|GetMaterial (Variables|Default|GetStaticMesh) 0) "M_MuscleMaterial" :!class /Script/Engine.PrimitiveComponent))
  (Variables|Materials|SetDynamicMaterial _returnvalue_2)
  (Components|Timeline|SetPlayRate (Variables|Default|GetFeedbackUpdate) (/ 1.0 (Variables|Materials|GetColorUpdateDuration)))
  (Components|Timeline|SetNewTime (Variables|Default|GetFeedbackUpdate) (Math|Float|SelectFloat 1.0 0.0 (Variables|Deformation|GetIsSolid))))

(event EventOnActorAbove
  (params (Actor :type Actor%20Object%20Reference))
  (Physics|HitMuscle Actor))

(event EventTrigger
  (Interaction|ToggleMuscleSolidity))

(event EventSetLock
  (params (state :type Boolean))
  (if (!= (Variables|Deformation|GetIsSolid) (Variables|Deformation|GetDefaultSolidityState))
    (CallFunction|Trigger)
    (if state
      (Variables|WeakZone|SetIsLocked true)
      (else
        (Variables|WeakZone|SetIsLocked false)))))

(fn ConstructionScript
  (Variables|Dimensions|SetCurrentScaleZ (Utilities|Struct|BreakFloatRangeBound (Utilities|Struct|BreakFloatRange (Variables|Dimensions|GetMeshHeight))))
  (Components|StaticMesh|SetStaticMesh (Variables|Default|GetStaticMesh) (Variables|Dimensions|GetMuscleMesh))
  (Deformation|RebuildMesh)
  (Utilities|IsValid (Variables|Materials|GetDynamicMaterial)
    (:Is%20Not%20Valid
      (bind _returnvalue (Rendering|Material|CreateDynamicMaterialInstance (Variables|Default|GetStaticMesh) 0 (Rendering|Material|GetMaterial (Variables|Default|GetStaticMesh) 0) "M_MuscleMaterial" :!class /Script/Engine.PrimitiveComponent))
      (bind _output_get (Variables|Materials|SetDynamicMaterial _returnvalue))
      (Rendering|Material|SetScalarParameterValue _output_get "LerpValue" (Math|Float|SelectFloat 0.0 1.0 (Variables|Deformation|GetIsSolid)) :!class /Script/Engine.MaterialInstanceDynamic))))

(fn RebuildMesh
  (bind _meshsize (Variables|Dimensions|GetMeshSize))
  (bind _staticmesh (Variables|Default|GetStaticMesh))
  (bind (_x _y) (Math|Vector2D|BreakVector2D _meshsize))
  (bind _staticmesh_2 (Variables|/Script/Engine.StaticMeshComponent|GetStaticMesh _staticmesh))
  (bind _returnvalue (StaticMesh|GetBoundingBox _staticmesh_2))
  (bind (_min _max) (Utilities|Struct|BreakBox _returnvalue))
  (Transformation|SetRelativeScale3D (Variables|Default|GetStaticMesh) (Math|Vector|MakeVector _x _y (Variables|Dimensions|GetCurrentScaleZ)))
  (Components|Box|SetBoxExtent (Variables|Default|GetAboveMeshCheck) (+ (* (- _max _min) (Variables|/Script/Engine.SceneComponent|GetRelativeScale3D (Variables|Default|GetStaticMesh)) 0.5) (Variables|Deformation|GetBoxSizeReduction)) false)
  (LocalVariables|SetAboveMuscleRelativeLocation (Math|Vector|MakeVector 0.0 0.0 (/ (.Z (Math|Vector|BreakVector (Variables|/Script/Engine.BoxComponent|GetBoxExtent (Variables|Default|GetAboveMeshCheck)))) (Variables|Dimensions|GetCurrentScaleZ))))
  (Transformation|SetRelativeLocation (Variables|Default|GetAboveMeshCheck) (LocalVariables|GetAboveMuscleRelativeLocation) false false)
  (Transformation|SetRelativeLocation (Variables|Default|GetDirection) (LocalVariables|GetAboveMuscleRelativeLocation) false false))

(fn DeformMesh
  (params (DeltaTime :type Float%20%28double-precision%29%20%28by%20ref%29))
  (if (and (Variables|Deformation|GetTriggerDeformation) (not (Variables|Deformation|GetIsSolid)))
    (LocalVariables|SetOriginalScaleZ (Variables|Dimensions|GetCurrentScaleZ))
    (Variables|Deformation|SetDeformationAlpha (Math|Float|Clamp(Float) (+ (* DeltaTime (Variables|Deformation|GetDeformationDirection) (Variables|Deformation|GetDeformationSpeed)) (Variables|Deformation|GetDeformationAlpha)) 0.0 (Variables|Deformation|GetDeformationDuration)))
    (bind _output_get (Variables|Dimensions|SetCurrentScaleZ (Math|Float|Lerp (Utilities|Struct|BreakFloatRangeBound (Utilities|Struct|BreakFloatRange (Variables|Dimensions|GetMeshHeight))) (Utilities|Struct|BreakFloatRangeBound (Utilities|Struct|BreakFloatRange (Variables|Dimensions|GetMeshHeight))) (Math|Curves|GetFloatValue (Variables|Deformation|GetDeformationCurve) (Math|Float|NormalizetoRange (Variables|Deformation|GetDeformationAlpha) 0.0 (Variables|Deformation|GetDeformationDuration))))))
    (Variables|Dimensions|SetCurrentScaleZ (Math|Float|SelectFloat (Variables|Deformation|GetMinScalePossible) (Variables|Dimensions|GetCurrentScaleZ) (<= _output_get (Variables|Deformation|GetMinScalePossible))))
    (Deformation|RebuildMesh)
    (Physics|MoveActors (- (LocalVariables|GetOriginalScaleZ) (Variables|Dimensions|GetCurrentScaleZ)))
    (if (or (== (Variables|Deformation|GetDeformationAlpha) 0.0) (== (Variables|Deformation|GetDeformationAlpha) (Variables|Deformation|GetDeformationDuration)))
      (Variables|Deformation|SetTriggerDeformation false)
      (if (Variables|Physics|GetShouldLaunchActors)
        (if (== (Variables|Deformation|GetDeformationDirection) 1)
          (Physics|LaunchActors)
          (CallFunction|EndDeformation)
          (else
            (CallFunction|EndDeformation)))))
    (elif (Math|Boolean|ANDBoolean (Deformation|IsDeformed) (not (Physics|IsSomethingAbove)) (not (Variables|Physics|GetShouldLaunchActors)))
      (CallFunction|EndDeformation))))

(fn LaunchActors
  (bind _keys (Utilities|Map|Keys (Variables|Physics|GetAboveActors)))
  (for _array_element _keys
    (LocalVariables|SetCurrentActor _array_element)
    (LocalVariables|SetCurrentVelocity (.Value (Utilities|Map|Find (Variables|Physics|GetAboveActors) (LocalVariables|GetCurrentActor))))
    (bind _asfirst_person_character (Utilities|Casting|CastToFirstPersonCharacter (LocalVariables|GetCurrentActor))
      (:then
        (bind _output_get (LocalVariables|SetCurrentCharacterMovement (Variables|/Script/Engine.Character|GetCharacterMovement _asfirst_person_character)))
        (Pawn|Components|CharacterMovement|SetMovementMode _output_get "MOVE_Falling" 0)
        (Variables|/Script/Engine.MovementComponent|SetVelocity (LocalVariables|GetCurrentCharacterMovement) (LocalVariables|GetCurrentVelocity))
        (Class|CharacterStateMachine|ChangeState (Variables|/Script/PROTOProfondeurs.FirstPersonCharacter|GetStateMachine _asfirst_person_character) "Fall"))
      (:CastFailed
        (if (Physics|IsSimulatingPhysics (Variables|/Script/Engine.Actor|GetRootComponent (LocalVariables|GetCurrentActor)) "None")
          (bind _asprimitive_component (Utilities|Casting|CastToPrimitiveComponent (Variables|/Script/Engine.Actor|GetRootComponent (LocalVariables|GetCurrentActor))))
          (Physics|AddForce _asprimitive_component (LocalVariables|GetCurrentVelocity) "None" false)))))
  (Utilities|Map|Clear (Variables|Physics|GetAboveActors))
  (Variables|Physics|SetShouldLaunchActors false))

(fn ResizeMeshCheck
  (bind _staticmesh (Variables|Default|GetStaticMesh))
  (bind _meshsize (Variables|Dimensions|GetMeshSize))
  (bind (_x _y) (Math|Vector2D|BreakVector2D _meshsize))
  (bind _relativelocation (Variables|/Script/Engine.SceneComponent|GetRelativeLocation _staticmesh))
  (bind (_x_2 _y_2 _z) (Math|Vector|BreakVector _relativelocation))
  (Transformation|SetRelativeLocation (Variables|Default|GetAboveMeshCheck) (Math|Vector|MakeVector _x_2 _y_2 (+ _z (Variables|Dimensions|GetCurrentScaleZ) (/ (Variables|Physics|GetTraceHeight) 2.0))) false false)
  (Components|Box|SetBoxExtent (Variables|Default|GetAboveMeshCheck) (/ (Math|Vector|MakeVector _x _y (Variables|Physics|GetTraceHeight)) 2) false))

(fn HitMuscle
  (params (HitActor :type Actor%20Object%20Reference))
  (bind _asbp_first_person_character (Utilities|Casting|CastToBP_FirstPersonCharacter HitActor))
  (bind _charactermovement (Variables|/Script/Engine.Character|GetCharacterMovement _asbp_first_person_character))
  (if (Variables|Deformation|GetIsSolid)
    (Class|PrimitiveComponent|SetPhysMaterialOverride (Variables|Default|GetStaticMesh) (Variables|Physics|GetSolidPhysicMaterial))
    (elif (not (Variables|Deformation|GetTriggerDeformation))
      (LocalVariables|SetActorVelocity (Math|Vector|VectorLength (Transformation|GetVelocity HitActor)))
      (bind _output_get (Variables|Physics|SetShouldLaunchActors (and (> (LocalVariables|GetActorVelocity) (Variables|Physics|GetMinVelocity)) (Collision|IsOverlappingActor (Variables|Default|GetAboveMeshCheck) HitActor :!class /Script/Engine.PrimitiveComponent))))
      (if _output_get
        (Utilities|Map|Add (Variables|Physics|GetAboveActors) HitActor (* (Math|Vector|GetUpVector (Variables|Default|GetStaticMesh)) (Math|Float|SelectFloat (Variables|Physics|GetFixedVelocity) (* (LocalVariables|GetActorVelocity) (Variables|Physics|GetVelocityMultiplier)) (Variables|Physics|GetUseFixedVelocity))))
        (Class|PrimitiveComponent|SetPhysMaterialOverride (Variables|Default|GetStaticMesh) (Variables|Physics|GetSolidPhysicMaterial))
        (CallFunction|StartDeformation)
        (Variables|/Script/Engine.MovementComponent|SetVelocity _charactermovement "0, 0, 0")
        (Variables|/Script/Engine.CharacterMovementComponent|SetGravityScale _charactermovement 0.0)
        (else
          (Class|PrimitiveComponent|SetPhysMaterialOverride (Variables|Default|GetStaticMesh) (Variables|Physics|GetSoftPhysicMaterial)))))))

(fn IsDeformed
  (return (!= (Variables|Dimensions|GetCurrentScaleZ) (Utilities|Struct|BreakFloatRangeBound (Utilities|Struct|BreakFloatRange (Variables|Dimensions|GetMeshHeight))))))

(fn IsSomethingAbove
  (bind _keys (Utilities|Map|Keys (Variables|Physics|GetAboveActors)))
  (for _array_element _keys
    (if (Collision|IsOverlappingActor (Variables|Default|GetAboveMeshCheck) _array_element :!class /Script/Engine.PrimitiveComponent)
      (return true)))
  (return false))

(fn UpdateMuscleSolidity
  (Class|PrimitiveComponent|SetPhysMaterialOverride (Variables|Default|GetStaticMesh) (select (Variables|Deformation|GetIsSolid) (Variables|Physics|GetSolidPhysicMaterial) (Variables|Physics|GetSoftPhysicMaterial)))
  (Interaction|UpdateInteraction)
  (Utilities|Time|ClearandInvalidateTimerbyHandle (Variables|Deformation|GetSolidityTimerHandle))
  (if (!= (Variables|Deformation|GetIsSolid) (Variables|Deformation|GetDefaultSolidityState))
    (bind _returnvalue (Utilities|Time|SetTimerbyEvent (EventDispatchers|CreateEvent :!event ToggleMuscleSolidity) (Variables|Deformation|GetSolidityDuration)))
    (Variables|Deformation|SetSolidityTimerHandle _returnvalue)))

(fn UpdateInteraction
  (Variables|/Script/PROTOProfondeurs.InteractableComponent|SetInteractionName (Variables|Default|GetInteractable) (Utilities|String|SelectText "Make soft" "Make solid" (Variables|Deformation|GetIsSolid))))

(fn ToggleMuscleSolidity
  (if (not (or (Variables|WeakZone|GetInWeakZone) (Variables|WeakZone|GetIsLocked)))
    (Variables|Deformation|SetIsSolid (not (Variables|Deformation|GetIsSolid)))
    (Interaction|UpdateMuscleSolidity)
    (CallFunction|UpdateColorFeedback)
    (CallFunction|UpdateBuzzer)))

(fn MoveActors
  (params (ScaleDiff :type Float%20%28double-precision%29%20%28by%20ref%29))
  (if (Variables|Physics|GetShouldLaunchActors)
    (bind _keys (Utilities|Map|Keys (Variables|Physics|GetAboveActors)))
    (for _array_element _keys
      (bind _output_get (LocalVariables|SetCurrentActor _array_element))
      (Transformation|SetActorLocation (LocalVariables|GetCurrentActor) (+ (Transformation|GetActorLocation _output_get) (* (* (Math|Vector|GetUpVector (Variables|Default|GetStaticMesh)) -1) (* (Variables|Dimensions|GetMeshZUnit) ScaleDiff))) false false))))