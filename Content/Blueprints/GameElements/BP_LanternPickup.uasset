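; Lantern pickup that floats and spins until the player interacts with it, then activates the character's lantern and tells the linked spike door to open.
; On pickup it hides the mesh, and a timeline fades assigned or tag-gathered lights from their cached intensities to zero, then destroys the actor.
; It also has a timeline event that lowers the door and a hook that writes its data to the world save.
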(event OnInteract(ENTInteractable)
  (params (Controller :type Player%20Controller%20Object%20Reference) (Pawn :type Pawn%20Object%20Reference) (InteractComponent :type Primitive%20Component%20Object%20Reference))
  (bind _asbp_first_person_character (Utilities|Casting|CastToBP_FirstPersonCharacter Pawn))
  (Class|ENTInteractableComponent|RemoveInteractable (Variables|Default|GetENTInteractable) (Variables|Default|GetLanternMesh))
  (Default|ActivateLantern _asbp_first_person_character true)
  (Components|Timeline|PlayfromStart (Variables|Default|GetLightsTimeline))
  (Rendering|SetVisibility (Variables|Default|GetLanternMesh) false true)
  (Class|ENTSpikeDoor|OpenDoor (Variables|Default|GetSpikeDoor)))

(event Custom|OpenDoor
  (Variables|Default|SetDoorInitPosition (Transformation|GetActorLocation (Variables|Default|GetSpikeDoor)))
  (bind _doorposition (Timeline|DoorTimeline Play)
    (:Update
      (Transformation|SetActorLocation (Variables|Default|GetSpikeDoor) (Math|Vector|MakeVector (.X (Math|Vector|BreakVector (Variables|Default|GetDoorInitPosition))) (.Y (Math|Vector|BreakVector (Variables|Default|GetDoorInitPosition))) (+ (Math|Float|Lerp 0.0 -1.4e+03 _doorposition) (.Z (Math|Vector|BreakVector (Variables|Default|GetDoorInitPosition))))) false false))))

(event EventSaveGameElementBP
  (params (CurrentWorldSave :type ENT%20World%20Save%20Object%20Reference))
  (Utilities|Map|Add (Variables|/Script/ENTSaves.ENTWorldSave|GetOtherElements CurrentWorldSave) (Variables|Default|GetSaveID) (Utilities|Struct|MakeENTGameElementData)))

(event EventTick
  (params (DeltaSeconds :type Float%20%28single-precision%29))
  (bind _lanterninitposition (Variables|Default|GetLanternInitPosition))
  (bind _lanternmesh (Variables|Default|GetLanternMesh))
  (bind (_x _y _z) (Math|Vector|BreakVector _lanterninitposition))
  (bind _relativerotation (Variables|/Script/Engine.SceneComponent|GetRelativeRotation _lanternmesh))
  (bind (_roll _pitch _yaw) (Math|Rotator|BreakRotator _relativerotation))
  (Transformation|SetRelativeRotation _lanternmesh (Math|Rotator|MakeRotator _roll _pitch (+ _yaw (* DeltaSeconds (Variables|Default|GetRotationSpeed)))) false false)
  (Transformation|SetRelativeLocation (Variables|Default|GetLanternMesh) (Math|Vector|MakeVector _x _y (+ _z (* (Math|Trig|Sin(Degrees) (* (Actor|GetGameTimeSinceCreation) (Variables|Default|GetFrequence))) (Variables|Default|GetAmplitude)))) false false))

(event EventBeginPlay
  (Components|Timeline|SetPlayRate (Variables|Default|GetLightsTimeline) (/ 1.0 (Variables|Ligths|GetFadeOutLightsDuration)))
  (Class|ENTInteractableComponent|AddInteractable (Variables|Default|GetENTInteractable) (Variables|Default|GetLanternMesh))
  (if (Utilities|Array|IsEmpty (Variables|Ligths|GetLights))
    (bind _outactors (Actor|GetAllActorsOfClasswithTag "/Script/Engine.Light" (Variables|Ligths|GetLanternLightTag)))
    (Variables|Ligths|SetLights _outactors))
  (for _array_element (Variables|Ligths|GetLights)
    (Utilities|Array|Add (Variables|Ligths|GetLightsDefaultIntensity) (Variables|/Script/Engine.LightComponentBase|GetIntensity (Variables|/Script/Engine.Light|GetLightComponent _array_element)))
    (Variables|Default|SetLanternInitPosition (Variables|/Script/Engine.SceneComponent|GetRelativeLocation (Variables|Default|GetLanternMesh)))))

(fn ConstructionScript)