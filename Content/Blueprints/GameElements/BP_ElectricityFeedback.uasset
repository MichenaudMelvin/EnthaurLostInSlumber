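; BP_ElectricityFeedback is an actor that shows an electricity post-process effect centered on its world location.
; Its construction script creates a dynamic instance of PPM_Electricity, assigns it as a weighted blendable to the Electricity post-process settings, and initializes its Radius and Position parameters.
; Tick pushes the Radius variable and actor location into the material each frame, so the effect follows changes to either.
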(event EventTick
  (params (DeltaSeconds :type Float%20%28single-precision%29))
  (Utilities|IsValid (Variables|Default|GetMaterial)
    (:Is%20Valid
      (Rendering|Material|SetScalarParameterValue (Variables|Default|GetMaterial) "Radius" (Variables|Default|GetRadius) :!class /Script/Engine.MaterialInstanceDynamic)
      (Rendering|Material|SetVectorParameterValue (Variables|Default|GetMaterial) "Position" (Math|Conversions|ToLinearColor(Vector) (Transformation|GetActorLocation)) :!class /Script/Engine.MaterialInstanceDynamic))))

(fn ConstructionScript
  (bind _returnvalue (Rendering|Material|CreateDynamicMaterialInstance "/Game/Art/PostProcess/PPM_Electricity.PPM_Electricity" "None" "None" :!class /Script/Engine.KismetMaterialLibrary))
  (bind _output_get (Variables|Default|SetMaterial _returnvalue))
  (Utilities|Array|SetArrayElem (Utilities|Struct|BreakWeightedBlendables (Utilities|Struct|BreakPostProcessSettings (Variables|/Script/Engine.PostProcessComponent|GetSettings (Variables|Default|GetElectricity)))) 0 (Utilities|Struct|MakeWeightedBlendable 1.0 _output_get))
  (Rendering|Material|SetScalarParameterValue (Variables|Default|GetMaterial) "Radius" (Variables|Default|GetValue) :!class /Script/Engine.MaterialInstanceDynamic)
  (Rendering|Material|SetVectorParameterValue (Variables|Default|GetMaterial) "Position" (Math|Conversions|ToLinearColor(Vector) (Transformation|GetActorLocation)) :!class /Script/Engine.MaterialInstanceDynamic))