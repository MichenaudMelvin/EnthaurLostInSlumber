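; BP_RespawnTree is a respawn tree actor that lights up through an emissive material parameter when activated.
; SetActive calls the parent logic, then plays EmissiveTimeline through its component reference, with the play rate set at BeginPlay from a configurable duration.
; The timeline update lerps Emissive from default to activation value.
; The construction script's node for setting the default emissive is unconnected.
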(event EventSetActive
  (|CallParentFunction)
  (Audio|Components|Audio|Play (Variables|Default|GetEmissiveTimeline)))

(event EventBeginPlay
  (Components|Timeline|SetPlayRate (Variables|Default|GetEmissiveTimeline) (/ 1.0 (Variables|Default|GetTimelineDurationDuration))))

(fn ConstructionScript)