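; Elevator actor whose button now triggers the ending cinematic and returns to the main menu.
; Interacting stops music, locks player states, hides the HUD and plays a level sequence, whose finish opens MainMenu.
; StartElevator, not called here, starts an up-then-down timeline ride with Wwise sounds and camera shake.
; Older two-floor travel logic is left unwired, though an overlap box still checks its timeline to lock jumping.
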(event OnInteract(Interactable)
  (params (Controller :type Player%20Controller%20Object%20Reference) (Pawn :type Pawn%20Object%20Reference) (InteractComponent :type Primitive%20Component%20Object%20Reference))
  (Default|StartMusic (.AsBP%20First%20Person%20Character (Utilities|Casting|CastToBP_FirstPersonCharacter (Game|Player|GetPlayerPawn 0))) "/Game/WwiseAudio/Events/Musics/AKE_Stop_Lvl_Chest.AKE_Stop_Lvl_Chest")
  (Class|AkGameplayStatics|PostEvent "/Game/WwiseAudio/Events/Musics/AKE_Stop_TitleScreen.AKE_Stop_TitleScreen")
  (Class|ENTCharacterStateMachine|LockAllStates (Variables|/Script/ENTCore.ENTDefaultCharacter|GetStateMachine (.AsENTDefault%20Character (Utilities|Casting|CastToENTDefaultCharacter Pawn))) true)
  (Class|ENTHUDManager|HideHUD (Subsystems|GetENTHUDManager))
  (Sequencer|Player|Play (Variables|Default|GetSequencePlayer) :!class /Script/MovieScene.MovieSceneSequencePlayer))

(event OnComponentBeginOverlap(JumpSaveBox)
  (params (OverlappedComponent :type Primitive%20Component%20Object%20Reference) (OtherActor :type Actor%20Object%20Reference) (OtherComp :type Primitive%20Component%20Object%20Reference) (OtherBodyIndex :type Integer) (bFromSweep :type Boolean) (SweepResult :type Hit%20Result%20Structure%20%28by%20ref%29))
  (if (Audio|Components|Audio|IsPlaying (Variables|Default|GetMoveElevator))
    (bind _asentdefault_character (Utilities|Casting|CastToENTDefaultCharacter OtherActor))
    (Class|ENTCharacterStateMachine|LockState (Variables|/Script/ENTCore.ENTDefaultCharacter|GetStateMachine _asentdefault_character) "Jump" true)))

(event OnComponentEndOverlap(JumpSaveBox)
  (params (OverlappedComponent :type Primitive%20Component%20Object%20Reference) (OtherActor :type Actor%20Object%20Reference) (OtherComp :type Primitive%20Component%20Object%20Reference) (OtherBodyIndex :type Integer))
  (bind _asentdefault_character (Utilities|Casting|CastToENTDefaultCharacter OtherActor))
  (Class|ENTCharacterStateMachine|LockState (Variables|/Script/ENTCore.ENTDefaultCharacter|GetStateMachine _asentdefault_character) "Jump" false))

(event Custom|StartElevator
  (Class|AkGameObject|PostAkEvent (Variables|Default|GetElevatorNoises) "/Game/WwiseAudio/Events/SFX/Gameplay/AKE_StartElevator.AKE_StartElevator")
  (Variables|Default|SetSpawnLocation (Transformation|GetActorLocation))
  (Class|ENTInteractableComponent|RemoveInteractable (Variables|Default|GetInteractable) (Variables|Default|GetFakeButton))
  (Components|Timeline|PlayfromStart (Variables|Default|GetTL_Up)))

(event Custom|FinishCinematic
  (Game|OpenLevel(byObjectReference) "/Game/Maps/MainMenu.MainMenu"))

(event EventBeginPlay
  (bind _returnvalue (Rendering|Material|CreateDynamicMaterialInstance "/Game/Art/GameElements/Elevator/Materials/M_ElevatorStele.M_ElevatorStele" "None" "None" :!class /Script/Engine.KismetMaterialLibrary))
  (Rendering|Material|SetMaterial (Variables|Default|GetStele) 0 _returnvalue)
  (Variables|Default|SetMaterial _returnvalue)
  (Class|ENTInteractableComponent|AddInteractable (Variables|Default|GetInteractable) (Variables|Default|GetFakeButton))
  (bind _returnvalue_2 (Sequencer|Player|CreateLevelSequencePlayer (Variables|Default|GetSequence) (Utilities|Struct|MakeMovieSceneSequencePlaybackSettings)))
  (bind _output_get (Variables|Default|SetSequencePlayer _returnvalue_2))
  (Utilities|IsValid 0
    (:Is%20Valid
      (EventDispatchers|BindEventtoOnFinished _output_get (EventDispatchers|CreateEvent :!event Custom|FinishCinematic)))))

(fn ConstructionScript)