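; Muscle game element that visually signals whether it is rigid or soft through particle and material colors.
; The construction script sets initial colors from IsSolid and passes ParticlesPath spline points to the direction particles as a Niagara vector array.
; On state change, it recolors both particle systems, restarts the interaction particles and fades SpikeInteraction's material colors through a timeline.
; The first completed fade also activates the direction particles.
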(event Custom|OnMuscleStateChange_Event
  (params (isSolid :type Boolean))
  (if isSolid
    (Niagara|SetNiagaraVariable(LinearColor) (Variables|Default|GetDirectionParticles) "ColorMin" (Variables|Particles|GetColorMinRigid))
    (Niagara|SetNiagaraVariable(LinearColor) (Variables|Default|GetDirectionParticles) "ColorMax" (Variables|Particles|GetColorMaxRigid))
    (Niagara|SetNiagaraVariable(LinearColor) (Variables|Default|GetInteractionParticles) "ColorMin" (Variables|Particles|GetColorMinRigid))
    (Niagara|SetNiagaraVariable(LinearColor) (Variables|Default|GetInteractionParticles) "ColorMax" (Variables|Particles|GetColorMaxRigid))
    (Niagara|ReinitializeSystem (Variables|Default|GetInteractionParticles))
    (Variables|Particles|SetBaseColor (Variables|Particles|GetColorMaxSoft))
    (bind _alpha (Timeline|ChangeColor PlayFromStart)
      (:Update
        (if isSolid
          (Rendering|Material|SetColorParameterValueonMaterials (Variables|Default|GetSpikeInteraction) "ColorMax" (Math|Color|Lerp(LinearColor) (Variables|Particles|GetBaseColor) (Variables|Particles|GetColorMaxRigid) _alpha))
          (Rendering|Material|SetColorParameterValueonMaterials (Variables|Default|GetSpikeInteraction) "ColorMin" (Math|Color|Lerp(LinearColor) (Variables|Particles|GetBaseColor) (Variables|Particles|GetColorMinRigid) _alpha))
          (else
            (Rendering|Material|SetColorParameterValueonMaterials (Variables|Default|GetSpikeInteraction) "ColorMax" (Math|Color|Lerp(LinearColor) (Variables|Particles|GetBaseColor) (Variables|Particles|GetColorMaxSoft) _alpha))
            (Rendering|Material|SetColorParameterValueonMaterials (Variables|Default|GetSpikeInteraction) "ColorMin" (Math|Color|Lerp(LinearColor) (Variables|Particles|GetBaseColor) (Variables|Particles|GetColorMinSoft) _alpha)))))
      (:Finished
        (Utilities|FlowControl|DoOnce false
          (:Completed
            (Components|Activation|Activate (Variables|Default|GetDirectionParticles) false)))))
    (else
      (Niagara|SetNiagaraVariable(LinearColor) (Variables|Default|GetDirectionParticles) "ColorMin" (Variables|Particles|GetColorMinSoft))
      (Niagara|SetNiagaraVariable(LinearColor) (Variables|Default|GetDirectionParticles) "ColorMax" (Variables|Particles|GetColorMaxSoft))
      (Niagara|SetNiagaraVariable(LinearColor) (Variables|Default|GetInteractionParticles) "ColorMin" (Variables|Particles|GetColorMinSoft))
      (Niagara|SetNiagaraVariable(LinearColor) (Variables|Default|GetInteractionParticles) "ColorMax" (Variables|Particles|GetColorMaxSoft))
      (Niagara|ReinitializeSystem (Variables|Default|GetInteractionParticles))
      (Variables|Particles|SetBaseColor (Variables|Particles|GetColorMaxRigid))
      (Timeline|ChangeColor PlayFromStart))))

(event EventBeginPlay
  (EventDispatchers|AssignOnMuscleStateChange (EventDispatchers|CreateEvent :!event Custom|OnMuscleStateChange_Event)))

(fn ConstructionScript
  (Transformation|SetWorldLocation (Variables|Default|GetDirectionParticles) (Spline|GetLocationatSplinePoint (Variables|Default|GetParticlesPath) 0 "World") false false)
  (Utilities|Array|Clear (Variables|Particles|GetParticulesDirectionLocations))
  (for _index (range 0 (- (Spline|GetNumberOfSplinePoints (Variables|Default|GetParticlesPath)) 1))
    (Utilities|Array|Add (Variables|Particles|GetParticulesDirectionLocations) (Spline|GetLocationatSplinePoint (Variables|Default|GetParticlesPath) _index "World")))
  (Class|NiagaraDataInterfaceArrayFunctionLibrary|SetNiagaraArrayVector (Variables|Default|GetDirectionParticles) "SequencialArray" (Variables|Particles|GetParticulesDirectionLocations))
  (Rendering|Material|SetColorParameterValueonMaterials (Variables|Default|GetSpikeInteraction) "ColorMin" (Math|Color|SelectColor (Variables|Particles|GetColorMinRigid) (Variables|Particles|GetColorMinSoft) (Variables|Default|GetbIsSolid)))
  (Rendering|Material|SetColorParameterValueonMaterials (Variables|Default|GetSpikeInteraction) "ColorMax" (Math|Color|SelectColor (Variables|Particles|GetColorMaxRigid) (Variables|Particles|GetColorMaxSoft) (Variables|Default|GetbIsSolid)))
  (Niagara|SetNiagaraVariable(LinearColor) (Variables|Default|GetDirectionParticles) "ColorMin" (Math|Color|SelectColor (Variables|Particles|GetColorMinRigid) (Variables|Particles|GetColorMinSoft) (Variables|Default|GetbIsSolid)))
  (Niagara|SetNiagaraVariable(LinearColor) (Variables|Default|GetDirectionParticles) "ColorMax" (Math|Color|SelectColor (Variables|Particles|GetColorMaxRigid) (Variables|Particles|GetColorMaxSoft) (Variables|Default|GetbIsSolid)))
  (Niagara|SetNiagaraVariable(LinearColor) (Variables|Default|GetInteractionParticles) "ColorMin" (Math|Color|SelectColor (Variables|Particles|GetColorMinRigid) (Variables|Particles|GetColorMinSoft) (Variables|Default|GetbIsSolid)))
  (Niagara|SetNiagaraVariable(LinearColor) (Variables|Default|GetInteractionParticles) "ColorMax" (Math|Color|SelectColor (Variables|Particles|GetColorMaxRigid) (Variables|Particles|GetColorMaxSoft) (Variables|Default|GetbIsSolid))))