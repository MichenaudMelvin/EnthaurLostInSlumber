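; BP_DebugTP is a debug teleport actor that moves the player pawn to a preset transform when a configured key is pressed.
; The construction script places a capsule at TargetTransform relative to its parent, marking the destination.
; On BeginPlay it enables input from player controller 0 and caches that player's pawn.
; An any-key handler compares the pressed key to DebugKey, then applies the capsule's world transform to the pawn without sweeping.
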(event EventBeginPlay
  (Input|EnableInput (Game|GetPlayerController 0))
  (Variables|Default|SetPawn (Game|Player|GetPlayerPawn 0)))

(event Input|KeyboardEvents|AnyKey
  (params (Key :type Key%20Structure :default "None"))
  (:Pressed
    (if (== Key (Variables|Default|GetDebugKey))
      (Transformation|SetActorTransform (Variables|Default|GetPawn) (Transformation|GetWorldTransform (Variables|Default|GetCapsule))))))

(fn ConstructionScript
  (Transformation|SetRelativeTransform (Variables|Default|GetCapsule) (Variables|Default|GetTargetTransform) false false))